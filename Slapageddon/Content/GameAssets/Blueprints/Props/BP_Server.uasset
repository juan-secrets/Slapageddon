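; BP_Server is a prop actor that slides over a table and throws randomly chosen tableware.
; After a delay on BeginPlay, Serve moves it by timeline lerp to an offset position, while an event track spawns random plates, cups, knives and forks at spawn points.
; When the move finishes, it launches the spawned items with randomized impulses, clears the list, and a second timeline slides it back to its start.
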(event Custom|Serve
  ;[0.15 0.15 0.15 0.5] Server comes over the table and throws all randomly created items
  (Transformation|SetActorLocation (Variables|Default|GetStartPosition) false false)
  (bind _newtrack_0 (Timeline|Timeline Play)
    (:Update
      (Transformation|SetActorLocation (Math|Vector|Lerp(Vector) (Variables|Default|GetStartPosition) (Variables|Default|GetEndPosition) _newtrack_0) false false))
    (:Finished
      (Utilities|FlowControl|Delay 1.0)
      (for _array_element (Variables|Default|GetServedItems)
        (Physics|AddImpulse (Actor|GetComponentbyClass _array_element "/Script/Engine.StaticMeshComponent") (Math|Vector|MakeVector (Math|Random|RandomFloatinRange -2e+02 -4.5e+02) (Math|Random|RandomFloatinRange 2e+02 4.5e+02) (Math|Random|RandomFloatinRange 5e+02 7.5e+02)) "None" false))
      (Utilities|FlowControl|Delay 0.5)
      (Utilities|Array|Clear (Variables|Default|GetServedItems))
      (CallFunction|LeaveTable))
    (:SpawnEvent
      (for _index (range 0 8)
        (switch int (Math|Random|RandomIntegerinRange 0 3)
          (:Default
            (bind _returnvalue (Game|SpawnActorfromClass "/Game/GameAssets/Blueprints/Props/BP_PropCup.BP_PropCup_C" (Math|Conversions|ToTransform(Vector) (Transformation|GetWorldLocation (Variables|Default|GetSpawnPoint1))) "Undefined" "MultiplyWithRoot" 0 0 :!label _label))
            (Utilities|Array|Add (Variables|Default|GetServedItems) _returnvalue))
          (:0
            (bind _returnvalue_2 (Game|SpawnActorfromClass "/Game/GameAssets/Blueprints/Props/BP_PropPlate.BP_PropPlate_C" (Math|Conversions|ToTransform(Vector) (Transformation|GetWorldLocation (Variables|Default|GetSpawnPoint))) "Undefined" "MultiplyWithRoot" 0 0))
            (Utilities|Array|Add (Variables|Default|GetServedItems) _returnvalue_2))
          (:1
            (goto _label))
          (:2
            (bind _returnvalue_3 (Game|SpawnActorfromClass "/Game/GameAssets/Blueprints/Props/BP_PropKnife.BP_PropKnife_C" (Math|Conversions|ToTransform(Vector) (Transformation|GetWorldLocation (Variables|Default|GetSpawnPoint2))) "Undefined" "MultiplyWithRoot" 0 0))
            (Utilities|Array|Add (Variables|Default|GetServedItems) _returnvalue_3))
          (:3
            (bind _returnvalue_4 (Game|SpawnActorfromClass "/Game/GameAssets/Blueprints/Props/BP_PropFork.BP_PropFork_C" (Math|Conversions|ToTransform(Vector) (Transformation|GetWorldLocation (Variables|Default|GetSpawnPoint3))) "Undefined" "MultiplyWithRoot" 0 0))
            (Utilities|Array|Add (Variables|Default|GetServedItems) _returnvalue_4)))))))

(event Custom|LeaveTable
  ;[0.15 0.15 0.15 0.5] Move the plate back off screen
  (bind _newtrack_0 (Timeline|Timeline_0 Play)
    (:Update
      (Transformation|SetActorLocation (Math|Vector|Lerp(Vector) (Variables|Default|GetEndPosition) (Variables|Default|GetStartPosition) _newtrack_0) false false))))

(event EventBeginPlay
  ;[0.15 0.15 0.15 0.5] Set Start and end location
  (bind _output_get (Variables|Default|SetStartPosition (Transformation|GetWorldLocation (Variables|Default|GetStaticMesh self))))
  (Variables|Default|SetEndPosition (Math|Vector|MakeVector (+ (.x _output_get) -75.0) (+ (.y _output_get) 75.0) (.z _output_get)))
  (Utilities|FlowControl|Delay 5.0)
  (CallFunction|Serve))

(fn ConstructionScript)