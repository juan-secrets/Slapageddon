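; Playing card actor that holds a suit and rank, shows the matching face, and animates its own movement and flipping.
; UpdateCard swaps the face texture on a dynamic material through UpdateBetterMaterialTexture (Deck2 art); the Deck1 variant is not called here.
; Move, scatter, flip and orient events only set target transforms, raising Z by deck size times card thickness for stacking.
; Tick eases location toward the target and rotates at constant speed.
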(event Custom|UpdateCard
  (params (NewSuit :type E_CardSuit%20Enum :default "NewEnumerator0") (NewRank :type E_CardRank%20Enum :default "NewEnumerator0"))
  (Variables|Default|SetSuit NewSuit)
  (Variables|Default|SetRank NewRank)
  (CallFunction|UpdateBetterMaterialTexture))

(event Custom|MoveToPosition
  (params (NewLocation :type Vector) (DeckSize :type Integer))
  ;[0.15 0.15 0.15 0.5] Card Movement Events
  (Variables|Default|SetTargetLocation (Math|Vector|MakeVector (.x NewLocation) (.y NewLocation) (+ (.z NewLocation) (* DeckSize (Variables|Default|GetCardThickness))))))

(event Custom|FlipCardUp
  ;[0.15 0.15 0.15 0.5] Card Movement Events
  (Variables|Default|SetTargetRotation (Math|Rotator|MakeRotator 0.0 0.0 (.yaw (Variables|Default|GetTargetRotation)))))

(event Custom|FlipCardDown
  ;[0.15 0.15 0.15 0.5] Card Movement Events
  (Variables|Default|SetTargetRotation (Math|Rotator|MakeRotator 1.8e+02 0.0 (.yaw (Variables|Default|GetTargetRotation)))))

(event Custom|RandomRotation
  ;[0.15 0.15 0.15 0.5] Card Movement Events
  (Variables|Default|SetTargetRotation (Math|Rotator|MakeRotator (.roll (Variables|Default|GetTargetRotation)) 0.0 (Math|Random|RandomFloatinRange -1.8e+02 1.8e+02))))

(event Custom|OrientToLocation
  (params (Start :type Vector) (Target :type Vector))
  ;[0.15 0.15 0.15 0.5] Card Movement Events
  (Variables|Default|SetTargetRotation (Math|Rotator|MakeRotator (.roll (Variables|Default|GetTargetRotation)) 0.0 (.yaw (Math|Rotator|FindLookatRotation Start Target)))))

(event Custom|RandomLocationAroundPoint
  (params (Location :type Vector) (MaxAround :type Float%20%28double-precision%29) (DeckSize :type Integer))
  ;[0.15 0.15 0.15 0.5] Card Movement Events
  (CallFunction|MovetoPosition (Math|Vector|MakeVector (+ (Math|Random|RandomFloatinRange (* MaxAround -1.0) MaxAround) (.x Location)) (+ (.y Location) (Math|Random|RandomFloatinRange (* MaxAround -1.0) MaxAround)) (.z Location)) DeckSize))

(event EventBeginPlay
  (bind _returnvalue (Rendering|Material|CreateDynamicMaterialInstance "/Game/GameAssets/Assets/Materials/M_CardFace.M_CardFace" "None" "None" :!class /Script/Engine.KismetMaterialLibrary))
  (bind _output_get (Variables|Default|SetCardFaceMaterial _returnvalue))
  (Rendering|Material|SetMaterial (Variables|Default|GetCardFace) 0 _output_get))

(event EventTick
  (params (DeltaSeconds :type Float%20%28single-precision%29))
  (bind _returnvalue (Transformation|GetActorLocation))
  (bind _targetlocation (Variables|Default|GetTargetLocation))
  (Utilities|FlowControl|Sequence
    (:then_0
      ;[0.15 0.15 0.15 0.5] Update Card Location
      (Transformation|SetActorLocation (Math|Vector|MakeVector (Math|Interpolation|FInterpTo (.x _returnvalue) (.x _targetlocation) DeltaSeconds (Variables|Default|GetMovingSpeed)) (Math|Interpolation|FInterpTo (.y _returnvalue) (.y _targetlocation) DeltaSeconds (Variables|Default|GetMovingSpeed)) (Math|Interpolation|FInterpTo (.z _returnvalue) (.z _targetlocation) DeltaSeconds (Variables|Default|GetMovingSpeed))) false false))
    (:then_1
      ;[0.15 0.15 0.15 0.5] Update Card Rotation
      (Transformation|SetActorRotation (Class|KismetMathLibrary|RInterptoConstant (Transformation|GetActorRotation) (Variables|Default|GetTargetRotation) DeltaSeconds (Variables|Default|GetRotationSpeed))))))

(fn ConstructionScript)

(fn ToString
  (switch Utilities|FlowControl|Switch|SwitchonE_CardSuit (Variables|Default|GetSuit)
    (:NewEnumerator0
      (LocalVariables|SetSuitString "Spade"))
    (:NewEnumerator1
      (LocalVariables|SetSuitString "Club"))
    (:NewEnumerator2
      (LocalVariables|SetSuitString "Heart"))
    (:NewEnumerator3
      (LocalVariables|SetSuitString "Diamond")))
  (switch Utilities|FlowControl|Switch|SwitchonE_CardRank (Variables|Default|GetRank)
    (:NewEnumerator0
      (LocalVariables|SetRankString "Ace"))
    (:NewEnumerator1
      (LocalVariables|SetRankString "2"))
    (:NewEnumerator2
      (LocalVariables|SetRankString "3"))
    (:NewEnumerator3
      (LocalVariables|SetRankString "4"))
    (:NewEnumerator4
      (LocalVariables|SetRankString "5"))
    (:NewEnumerator5
      (LocalVariables|SetRankString "6"))
    (:NewEnumerator6
      (LocalVariables|SetRankString "7"))
    (:NewEnumerator7
      (LocalVariables|SetRankString "8"))
    (:NewEnumerator8
      (LocalVariables|SetRankString "9"))
    (:NewEnumerator9
      (LocalVariables|SetRankString "10"))
    (:NewEnumerator10
      (LocalVariables|SetRankString "Jack"))
    (:NewEnumerator11
      (LocalVariables|SetRankString "Queen"))
    (:NewEnumerator12
      (LocalVariables|SetRankString "King")))
  (return (Utilities|String|Append (LocalVariables|GetRankString) " of " (LocalVariables|GetSuitString))))

(fn UpdateMaterialTexture
  (Utilities|FlowControl|Sequence
    (:then_0
      (switch Utilities|FlowControl|Switch|SwitchonE_CardSuit (Variables|Default|GetSuit)
        (:NewEnumerator0
          ;[0.15 0.15 0.15 0.5] Spades
          (switch Utilities|FlowControl|Switch|SwitchonE_CardRank (Variables|Default|GetRank)
            (:NewEnumerator0
              (LocalVariables|SetNewTexture "/Game/CardDeck/2ColorCards/726X1044/Deck1/T_2ColorCards_Deck1_HighRes_SpadesA_Diffuse.T_2ColorCards_Deck1_HighRes_SpadesA_Diffuse"))
            (:NewEnumerator1
              (LocalVariables|SetNewTexture "/Game/CardDeck/2ColorCards/726X1044/Deck1/T_2ColorCards_Deck1_HighRes_Spades2_Diffuse.T_2ColorCards_Deck1_HighRes_Spades2_Diffuse"))
            (:NewEnumerator2
              (LocalVariables|SetNewTexture "/Game/CardDeck/2ColorCards/726X1044/Deck1/T_2ColorCards_Deck1_HighRes_Spades3_Diffuse.T_2ColorCards_Deck1_HighRes_Spades3_Diffuse"))
            (:NewEnumerator3
              (LocalVariables|SetNewTexture "/Game/CardDeck/2ColorCards/726X1044/Deck1/T_2ColorCards_Deck1_HighRes_Spades4_Diffuse.T_2ColorCards_Deck1_HighRes_Spades4_Diffuse"))
            (:NewEnumerator4
              (LocalVariables|SetNewTexture "/Game/CardDeck/2ColorCards/726X1044/Deck1/T_2ColorCards_Deck1_HighRes_Spades5_Diffuse.T_2ColorCards_Deck1_HighRes_Spades5_Diffuse"))
            (:NewEnumerator5
              (LocalVariables|SetNewTexture "/Game/CardDeck/2ColorCards/726X1044/Deck1/T_2ColorCards_Deck1_HighRes_Spades6_Diffuse.T_2ColorCards_Deck1_HighRes_Spades6_Diffuse"))
            (:NewEnumerator6
              (LocalVariables|SetNewTexture "/Game/CardDeck/2ColorCards/726X1044/Deck1/T_2ColorCards_Deck1_HighRes_Spades7_Diffuse.T_2ColorCards_Deck1_HighRes_Spades7_Diffuse"))
            (:NewEnumerator7
              (LocalVariables|SetNewTexture "/Game/CardDeck/2ColorCards/726X1044/Deck1/T_2ColorCards_Deck1_HighRes_Spades8_Diffuse.T_2ColorCards_Deck1_HighRes_Spades8_Diffuse"))
            (:NewEnumerator8
              (LocalVariables|SetNewTexture "/Game/CardDeck/2ColorCards/726X1044/Deck1/T_2ColorCards_Deck1_HighRes_Spades9_Diffuse.T_2ColorCards_Deck1_HighRes_Spades9_Diffuse"))
            (:NewEnumerator9
              (LocalVariables|SetNewTexture "/Game/CardDeck/2ColorCards/726X1044/Deck1/T_2ColorCards_Deck1_HighRes_Spades10_Diffuse.T_2ColorCards_Deck1_HighRes_Spades10_Diffuse"))
            (:NewEnumerator10
              (LocalVariables|SetNewTexture "/Game/CardDeck/2ColorCards/726X1044/Deck1/T_2ColorCards_Deck1_HighRes_SpadesJ_Diffuse.T_2ColorCards_Deck1_HighRes_SpadesJ_Diffuse"))
            (:NewEnumerator11
              (LocalVariables|SetNewTexture "/Game/CardDeck/2ColorCards/726X1044/Deck1/T_2ColorCards_Deck1_HighRes_SpadesQ_Diffuse.T_2ColorCards_Deck1_HighRes_SpadesQ_Diffuse"))
            (:NewEnumerator12
              (LocalVariables|SetNewTexture "/Game/CardDeck/2ColorCards/726X1044/Deck1/T_2ColorCards_Deck1_HighRes_SpadesK_Diffuse.T_2ColorCards_Deck1_HighRes_SpadesK_Diffuse"))))
        (:NewEnumerator1
          ;[0.15 0.15 0.15 0.5] Clubs
          (switch Utilities|FlowControl|Switch|SwitchonE_CardRank (Variables|Default|GetRank)
            (:NewEnumerator0
              (LocalVariables|SetNewTexture "/Game/CardDeck/2ColorCards/726X1044/Deck1/T_2ColorCards_Deck1_HighRes_ClubsA_Diffuse.T_2ColorCards_Deck1_HighRes_ClubsA_Diffuse"))
            (:NewEnumerator1
              (LocalVariables|SetNewTexture "/Game/CardDeck/2ColorCards/726X1044/Deck1/T_2ColorCards_Deck1_HighRes_Clubs2_Diffuse.T_2ColorCards_Deck1_HighRes_Clubs2_Diffuse"))
            (:NewEnumerator2
              (LocalVariables|SetNewTexture "/Game/CardDeck/2ColorCards/726X1044/Deck1/T_2ColorCards_Deck1_HighRes_Clubs3_Diffuse.T_2ColorCards_Deck1_HighRes_Clubs3_Diffuse"))
            (:NewEnumerator3
              (LocalVariables|SetNewTexture "/Game/CardDeck/2ColorCards/726X1044/Deck1/T_2ColorCards_Deck1_HighRes_Clubs4_Diffuse.T_2ColorCards_Deck1_HighRes_Clubs4_Diffuse"))
            (:NewEnumerator4
              (LocalVariables|SetNewTexture "/Game/CardDeck/2ColorCards/726X1044/Deck1/T_2ColorCards_Deck1_HighRes_Clubs5_Diffuse.T_2ColorCards_Deck1_HighRes_Clubs5_Diffuse"))
            (:NewEnumerator5
              (LocalVariables|SetNewTexture "/Game/CardDeck/2ColorCards/726X1044/Deck1/T_2ColorCards_Deck1_HighRes_Clubs6_Diffuse.T_2ColorCards_Deck1_HighRes_Clubs6_Diffuse"))
            (:NewEnumerator6
              (LocalVariables|SetNewTexture "/Game/CardDeck/2ColorCards/726X1044/Deck1/T_2ColorCards_Deck1_HighRes_Clubs7_Diffuse.T_2ColorCards_Deck1_HighRes_Clubs7_Diffuse"))
            (:NewEnumerator7
              (LocalVariables|SetNewTexture "/Game/CardDeck/2ColorCards/726X1044/Deck1/T_2ColorCards_Deck1_HighRes_Clubs8_Diffuse.T_2ColorCards_Deck1_HighRes_Clubs8_Diffuse"))
            (:NewEnumerator8
              (LocalVariables|SetNewTexture "/Game/CardDeck/2ColorCards/726X1044/Deck1/T_2ColorCards_Deck1_HighRes_Clubs9_Diffuse.T_2ColorCards_Deck1_HighRes_Clubs9_Diffuse"))
            (:NewEnumerator9
              (LocalVariables|SetNewTexture "/Game/CardDeck/2ColorCards/726X1044/Deck1/T_2ColorCards_Deck1_HighRes_Clubs10_Diffuse.T_2ColorCards_Deck1_HighRes_Clubs10_Diffuse"))
            (:NewEnumerator10
              (LocalVariables|SetNewTexture "/Game/CardDeck/2ColorCards/726X1044/Deck1/T_2ColorCards_Deck1_HighRes_ClubsJ_Diffuse.T_2ColorCards_Deck1_HighRes_ClubsJ_Diffuse"))
            (:NewEnumerator11
              (LocalVariables|SetNewTexture "/Game/CardDeck/2ColorCards/726X1044/Deck1/T_2ColorCards_Deck1_HighRes_ClubsQ_Diffuse.T_2ColorCards_Deck1_HighRes_ClubsQ_Diffuse"))
            (:NewEnumerator12
              (LocalVariables|SetNewTexture "/Game/CardDeck/2ColorCards/726X1044/Deck1/T_2ColorCards_Deck1_HighRes_ClubsK_Diffuse.T_2ColorCards_Deck1_HighRes_ClubsK_Diffuse"))))
        (:NewEnumerator2
          ;[0.15 0.15 0.15 0.5] Hearts
          (switch Utilities|FlowControl|Switch|SwitchonE_CardRank (Variables|Default|GetRank)
            (:NewEnumerator0
              (LocalVariables|SetNewTexture "/Game/CardDeck/2ColorCards/726X1044/Deck1/T_2ColorCards_Deck1_HighRes_HeartsA_Diffuse.T_2ColorCards_Deck1_HighRes_HeartsA_Diffuse"))
            (:NewEnumerator1
              (LocalVariables|SetNewTexture "/Game/CardDeck/2ColorCards/726X1044/Deck1/T_2ColorCards_Deck1_HighRes_Hearts2_Diffuse.T_2ColorCards_Deck1_HighRes_Hearts2_Diffuse"))
            (:NewEnumerator2
              (LocalVariables|SetNewTexture "/Game/CardDeck/2ColorCards/726X1044/Deck1/T_2ColorCards_Deck1_HighRes_Hearts3_Diffuse.T_2ColorCards_Deck1_HighRes_Hearts3_Diffuse"))
            (:NewEnumerator3
              (LocalVariables|SetNewTexture "/Game/CardDeck/2ColorCards/726X1044/Deck1/T_2ColorCards_Deck1_HighRes_Hearts4_Diffuse.T_2ColorCards_Deck1_HighRes_Hearts4_Diffuse"))
            (:NewEnumerator4
              (LocalVariables|SetNewTexture "/Game/CardDeck/2ColorCards/726X1044/Deck1/T_2ColorCards_Deck1_HighRes_Hearts5_Diffuse.T_2ColorCards_Deck1_HighRes_Hearts5_Diffuse"))
            (:NewEnumerator5
              (LocalVariables|SetNewTexture "/Game/CardDeck/2ColorCards/726X1044/Deck1/T_2ColorCards_Deck1_HighRes_Hearts6_Diffuse.T_2ColorCards_Deck1_HighRes_Hearts6_Diffuse"))
            (:NewEnumerator6
              (LocalVariables|SetNewTexture "/Game/CardDeck/2ColorCards/726X1044/Deck1/T_2ColorCards_Deck1_HighRes_Hearts7_Diffuse.T_2ColorCards_Deck1_HighRes_Hearts7_Diffuse"))
            (:NewEnumerator7
              (LocalVariables|SetNewTexture "/Game/CardDeck/2ColorCards/726X1044/Deck1/T_2ColorCards_Deck1_HighRes_Hearts8_Diffuse.T_2ColorCards_Deck1_HighRes_Hearts8_Diffuse"))
            (:NewEnumerator8
              (LocalVariables|SetNewTexture "/Game/CardDeck/2ColorCards/726X1044/Deck1/T_2ColorCards_Deck1_HighRes_Hearts9_Diffuse.T_2ColorCards_Deck1_HighRes_Hearts9_Diffuse"))
            (:NewEnumerator9
              (LocalVariables|SetNewTexture "/Game/CardDeck/2ColorCards/726X1044/Deck1/T_2ColorCards_Deck1_HighRes_Hearts10_Diffuse.T_2ColorCards_Deck1_HighRes_Hearts10_Diffuse"))
            (:NewEnumerator10
              (LocalVariables|SetNewTexture "/Game/CardDeck/2ColorCards/726X1044/Deck1/T_2ColorCards_Deck1_HighRes_HeartsJ_Diffuse.T_2ColorCards_Deck1_HighRes_HeartsJ_Diffuse"))
            (:NewEnumerator11
              (LocalVariables|SetNewTexture "/Game/CardDeck/2ColorCards/726X1044/Deck1/T_2ColorCards_Deck1_HighRes_HeartsQ_Diffuse.T_2ColorCards_Deck1_HighRes_HeartsQ_Diffuse"))
            (:NewEnumerator12
              (LocalVariables|SetNewTexture "/Game/CardDeck/2ColorCards/726X1044/Deck1/T_2ColorCards_Deck1_HighRes_HeartsK_Diffuse.T_2ColorCards_Deck1_HighRes_HeartsK_Diffuse"))))
        (:NewEnumerator3
          ;[0.15 0.15 0.15 0.5] Diamonds
          (switch Utilities|FlowControl|Switch|SwitchonE_CardRank (Variables|Default|GetRank)
            (:NewEnumerator0
              (LocalVariables|SetNewTexture "/Game/CardDeck/2ColorCards/726X1044/Deck1/T_2ColorCards_Deck1_HighRes_DiamondsA_Diffuse.T_2ColorCards_Deck1_HighRes_DiamondsA_Diffuse"))
            (:NewEnumerator1
              (LocalVariables|SetNewTexture "/Game/CardDeck/2ColorCards/726X1044/Deck1/T_2ColorCards_Deck1_HighRes_Diamonds2_Diffuse.T_2ColorCards_Deck1_HighRes_Diamonds2_Diffuse"))
            (:NewEnumerator2
              (LocalVariables|SetNewTexture "/Game/CardDeck/2ColorCards/726X1044/Deck1/T_2ColorCards_Deck1_HighRes_Diamonds3_Diffuse.T_2ColorCards_Deck1_HighRes_Diamonds3_Diffuse"))
            (:NewEnumerator3
              (LocalVariables|SetNewTexture "/Game/CardDeck/2ColorCards/726X1044/Deck1/T_2ColorCards_Deck1_HighRes_Diamonds4_Diffuse.T_2ColorCards_Deck1_HighRes_Diamonds4_Diffuse"))
            (:NewEnumerator4
              (LocalVariables|SetNewTexture "/Game/CardDeck/2ColorCards/726X1044/Deck1/T_2ColorCards_Deck1_HighRes_Diamonds5_Diffuse.T_2ColorCards_Deck1_HighRes_Diamonds5_Diffuse"))
            (:NewEnumerator5
              (LocalVariables|SetNewTexture "/Game/CardDeck/2ColorCards/726X1044/Deck1/T_2ColorCards_Deck1_HighRes_Diamonds6_Diffuse.T_2ColorCards_Deck1_HighRes_Diamonds6_Diffuse"))
            (:NewEnumerator6
              (LocalVariables|SetNewTexture "/Game/CardDeck/2ColorCards/726X1044/Deck1/T_2ColorCards_Deck1_HighRes_Diamonds7_Diffuse.T_2ColorCards_Deck1_HighRes_Diamonds7_Diffuse"))
            (:NewEnumerator7
              (LocalVariables|SetNewTexture "/Game/CardDeck/2ColorCards/726X1044/Deck1/T_2ColorCards_Deck1_HighRes_Diamonds8_Diffuse.T_2ColorCards_Deck1_HighRes_Diamonds8_Diffuse"))
            (:NewEnumerator8
              (LocalVariables|SetNewTexture "/Game/CardDeck/2ColorCards/726X1044/Deck1/T_2ColorCards_Deck1_HighRes_Diamonds9_Diffuse.T_2ColorCards_Deck1_HighRes_Diamonds9_Diffuse"))
            (:NewEnumerator9
              (LocalVariables|SetNewTexture "/Game/CardDeck/2ColorCards/726X1044/Deck1/T_2ColorCards_Deck1_HighRes_Diamonds10_Diffuse.T_2ColorCards_Deck1_HighRes_Diamonds10_Diffuse"))
            (:NewEnumerator10
              (LocalVariables|SetNewTexture "/Game/CardDeck/2ColorCards/726X1044/Deck1/T_2ColorCards_Deck1_HighRes_DiamondsJ_Diffuse.T_2ColorCards_Deck1_HighRes_DiamondsJ_Diffuse"))
            (:NewEnumerator11
              (LocalVariables|SetNewTexture "/Game/CardDeck/2ColorCards/726X1044/Deck1/T_2ColorCards_Deck1_HighRes_DiamondsQ_Diffuse.T_2ColorCards_Deck1_HighRes_DiamondsQ_Diffuse"))
            (:NewEnumerator12
              (LocalVariables|SetNewTexture "/Game/CardDeck/2ColorCards/726X1044/Deck1/T_2ColorCards_Deck1_HighRes_DiamondsK_Diffuse.T_2ColorCards_Deck1_HighRes_DiamondsK_Diffuse"))))))
    (:then_1
      (Rendering|Material|SetTextureParameterValue (Variables|Default|GetCardFaceMaterial) "CardFace_Texture" (LocalVariables|GetNewTexture)))))

(fn UpdateBetterMaterialTexture
  (Utilities|FlowControl|Sequence
    (:then_0
      (switch Utilities|FlowControl|Switch|SwitchonE_CardSuit (Variables|Default|GetSuit)
        (:NewEnumerator0
          ;[0.15 0.15 0.15 0.5] Spades
          (switch Utilities|FlowControl|Switch|SwitchonE_CardRank (Variables|Default|GetRank)
            (:NewEnumerator0
              (LocalVariables|SetNewTexture "/Game/CardDeck/2ColorCards/726X1044/Deck2/T_2ColorCards_Deck2_HighRes_SpadesA_Diffuse.T_2ColorCards_Deck2_HighRes_SpadesA_Diffuse"))
            (:NewEnumerator1
              (LocalVariables|SetNewTexture "/Game/CardDeck/2ColorCards/726X1044/Deck2/T_2ColorCards_Deck2_HighRes_Spades2_Diffuse.T_2ColorCards_Deck2_HighRes_Spades2_Diffuse"))
            (:NewEnumerator2
              (LocalVariables|SetNewTexture "/Game/CardDeck/2ColorCards/726X1044/Deck2/T_2ColorCards_Deck2_HighRes_Spades3_Diffuse.T_2ColorCards_Deck2_HighRes_Spades3_Diffuse"))
            (:NewEnumerator3
              (LocalVariables|SetNewTexture "/Game/CardDeck/2ColorCards/726X1044/Deck2/T_2ColorCards_Deck2_HighRes_Spades4_Diffuse.T_2ColorCards_Deck2_HighRes_Spades4_Diffuse"))
            (:NewEnumerator4
              (LocalVariables|SetNewTexture "/Game/CardDeck/2ColorCards/726X1044/Deck2/T_2ColorCards_Deck2_HighRes_Spades5_Diffuse.T_2ColorCards_Deck2_HighRes_Spades5_Diffuse"))
            (:NewEnumerator5
              (LocalVariables|SetNewTexture "/Game/CardDeck/2ColorCards/726X1044/Deck2/T_2ColorCards_Deck2_HighRes_Spades6_Diffuse.T_2ColorCards_Deck2_HighRes_Spades6_Diffuse"))
            (:NewEnumerator6
              (LocalVariables|SetNewTexture "/Game/CardDeck/2ColorCards/726X1044/Deck2/T_2ColorCards_Deck2_HighRes_Spades7_Diffuse.T_2ColorCards_Deck2_HighRes_Spades7_Diffuse"))
            (:NewEnumerator7
              (LocalVariables|SetNewTexture "/Game/CardDeck/2ColorCards/726X1044/Deck2/T_2ColorCards_Deck2_HighRes_Spades8_Diffuse.T_2ColorCards_Deck2_HighRes_Spades8_Diffuse"))
            (:NewEnumerator8
              (LocalVariables|SetNewTexture "/Game/CardDeck/2ColorCards/726X1044/Deck2/T_2ColorCards_Deck2_HighRes_Spades9_Diffuse.T_2ColorCards_Deck2_HighRes_Spades9_Diffuse"))
            (:NewEnumerator9
              (LocalVariables|SetNewTexture "/Game/CardDeck/2ColorCards/726X1044/Deck2/T_2ColorCards_Deck2_HighRes_Spades10_Diffuse.T_2ColorCards_Deck2_HighRes_Spades10_Diffuse"))
            (:NewEnumerator10
              (LocalVariables|SetNewTexture "/Game/CardDeck/2ColorCards/726X1044/Deck2/T_2ColorCards_Deck2_HighRes_SpadesJ_Diffuse.T_2ColorCards_Deck2_HighRes_SpadesJ_Diffuse"))
            (:NewEnumerator11
              (LocalVariables|SetNewTexture "/Game/CardDeck/2ColorCards/726X1044/Deck2/T_2ColorCards_Deck2_HighRes_SpadesQ_Diffuse.T_2ColorCards_Deck2_HighRes_SpadesQ_Diffuse"))
            (:NewEnumerator12
              (LocalVariables|SetNewTexture "/Game/CardDeck/2ColorCards/726X1044/Deck2/T_2ColorCards_Deck2_HighRes_SpadesK_Diffuse.T_2ColorCards_Deck2_HighRes_SpadesK_Diffuse"))))
        (:NewEnumerator1
          ;[0.15 0.15 0.15 0.5] Clubs
          (switch Utilities|FlowControl|Switch|SwitchonE_CardRank (Variables|Default|GetRank)
            (:NewEnumerator0
              (LocalVariables|SetNewTexture "/Game/CardDeck/2ColorCards/726X1044/Deck2/T_2ColorCards_Deck2_HighRes_ClubsA_Diffuse.T_2ColorCards_Deck2_HighRes_ClubsA_Diffuse"))
            (:NewEnumerator1
              (LocalVariables|SetNewTexture "/Game/CardDeck/2ColorCards/726X1044/Deck2/T_2ColorCards_Deck2_HighRes_Clubs2_Diffuse.T_2ColorCards_Deck2_HighRes_Clubs2_Diffuse"))
            (:NewEnumerator2
              (LocalVariables|SetNewTexture "/Game/CardDeck/2ColorCards/726X1044/Deck2/T_2ColorCards_Deck2_HighRes_Clubs3_Diffuse.T_2ColorCards_Deck2_HighRes_Clubs3_Diffuse"))
            (:NewEnumerator3
              (LocalVariables|SetNewTexture "/Game/CardDeck/2ColorCards/726X1044/Deck2/T_2ColorCards_Deck2_HighRes_Clubs4_Diffuse.T_2ColorCards_Deck2_HighRes_Clubs4_Diffuse"))
            (:NewEnumerator4
              (LocalVariables|SetNewTexture "/Game/CardDeck/2ColorCards/726X1044/Deck2/T_2ColorCards_Deck2_HighRes_Clubs5_Diffuse.T_2ColorCards_Deck2_HighRes_Clubs5_Diffuse"))
            (:NewEnumerator5
              (LocalVariables|SetNewTexture "/Game/CardDeck/2ColorCards/726X1044/Deck2/T_2ColorCards_Deck2_HighRes_Clubs6_Diffuse.T_2ColorCards_Deck2_HighRes_Clubs6_Diffuse"))
            (:NewEnumerator6
              (LocalVariables|SetNewTexture "/Game/CardDeck/2ColorCards/726X1044/Deck2/T_2ColorCards_Deck2_HighRes_Clubs7_Diffuse.T_2ColorCards_Deck2_HighRes_Clubs7_Diffuse"))
            (:NewEnumerator7
              (LocalVariables|SetNewTexture "/Game/CardDeck/2ColorCards/726X1044/Deck2/T_2ColorCards_Deck2_HighRes_Clubs8_Diffuse.T_2ColorCards_Deck2_HighRes_Clubs8_Diffuse"))
            (:NewEnumerator8
              (LocalVariables|SetNewTexture "/Game/CardDeck/2ColorCards/726X1044/Deck2/T_2ColorCards_Deck2_HighRes_Clubs9_Diffuse.T_2ColorCards_Deck2_HighRes_Clubs9_Diffuse"))
            (:NewEnumerator9
              (LocalVariables|SetNewTexture "/Game/CardDeck/2ColorCards/726X1044/Deck2/T_2ColorCards_Deck2_HighRes_Clubs10_Diffuse.T_2ColorCards_Deck2_HighRes_Clubs10_Diffuse"))
            (:NewEnumerator10
              (LocalVariables|SetNewTexture "/Game/CardDeck/2ColorCards/726X1044/Deck2/T_2ColorCards_Deck2_HighRes_ClubsJ_Diffuse.T_2ColorCards_Deck2_HighRes_ClubsJ_Diffuse"))
            (:NewEnumerator11
              (LocalVariables|SetNewTexture "/Game/CardDeck/2ColorCards/726X1044/Deck2/T_2ColorCards_Deck2_HighRes_ClubsQ_Diffuse.T_2ColorCards_Deck2_HighRes_ClubsQ_Diffuse"))
            (:NewEnumerator12
              (LocalVariables|SetNewTexture "/Game/CardDeck/2ColorCards/726X1044/Deck2/T_2ColorCards_Deck2_HighRes_ClubsK_Diffuse.T_2ColorCards_Deck2_HighRes_ClubsK_Diffuse"))))
        (:NewEnumerator2
          ;[0.15 0.15 0.15 0.5] Hearts
          (switch Utilities|FlowControl|Switch|SwitchonE_CardRank (Variables|Default|GetRank)
            (:NewEnumerator0
              (LocalVariables|SetNewTexture "/Game/CardDeck/2ColorCards/726X1044/Deck2/T_2ColorCards_Deck2_HighRes_HeartsA_Diffuse.T_2ColorCards_Deck2_HighRes_HeartsA_Diffuse"))
            (:NewEnumerator1
              (LocalVariables|SetNewTexture "/Game/CardDeck/2ColorCards/726X1044/Deck2/T_2ColorCards_Deck2_HighRes_Hearts2_Diffuse.T_2ColorCards_Deck2_HighRes_Hearts2_Diffuse"))
            (:NewEnumerator2
              (LocalVariables|SetNewTexture "/Game/CardDeck/2ColorCards/726X1044/Deck2/T_2ColorCards_Deck2_HighRes_Hearts3_Diffuse.T_2ColorCards_Deck2_HighRes_Hearts3_Diffuse"))
            (:NewEnumerator3
              (LocalVariables|SetNewTexture "/Game/CardDeck/2ColorCards/726X1044/Deck2/T_2ColorCards_Deck2_HighRes_Hearts4_Diffuse.T_2ColorCards_Deck2_HighRes_Hearts4_Diffuse"))
            (:NewEnumerator4
              (LocalVariables|SetNewTexture "/Game/CardDeck/2ColorCards/726X1044/Deck2/T_2ColorCards_Deck2_HighRes_Hearts5_Diffuse.T_2ColorCards_Deck2_HighRes_Hearts5_Diffuse"))
            (:NewEnumerator5
              (LocalVariables|SetNewTexture "/Game/CardDeck/2ColorCards/726X1044/Deck2/T_2ColorCards_Deck2_HighRes_Hearts6_Diffuse.T_2ColorCards_Deck2_HighRes_Hearts6_Diffuse"))
            (:NewEnumerator6
              (LocalVariables|SetNewTexture "/Game/CardDeck/2ColorCards/726X1044/Deck2/T_2ColorCards_Deck2_HighRes_Hearts7_Diffuse.T_2ColorCards_Deck2_HighRes_Hearts7_Diffuse"))
            (:NewEnumerator7
              (LocalVariables|SetNewTexture "/Game/CardDeck/2ColorCards/726X1044/Deck2/T_2ColorCards_Deck2_HighRes_Hearts8_Diffuse.T_2ColorCards_Deck2_HighRes_Hearts8_Diffuse"))
            (:NewEnumerator8
              (LocalVariables|SetNewTexture "/Game/CardDeck/2ColorCards/726X1044/Deck2/T_2ColorCards_Deck2_HighRes_Hearts9_Diffuse.T_2ColorCards_Deck2_HighRes_Hearts9_Diffuse"))
            (:NewEnumerator9
              (LocalVariables|SetNewTexture "/Game/CardDeck/2ColorCards/726X1044/Deck2/T_2ColorCards_Deck2_HighRes_Hearts10_Diffuse.T_2ColorCards_Deck2_HighRes_Hearts10_Diffuse"))
            (:NewEnumerator10
              (LocalVariables|SetNewTexture "/Game/CardDeck/2ColorCards/726X1044/Deck2/T_2ColorCards_Deck2_HighRes_HeartsJ_Diffuse.T_2ColorCards_Deck2_HighRes_HeartsJ_Diffuse"))
            (:NewEnumerator11
              (LocalVariables|SetNewTexture "/Game/CardDeck/2ColorCards/726X1044/Deck2/T_2ColorCards_Deck2_HighRes_HeartsQ_Diffuse.T_2ColorCards_Deck2_HighRes_HeartsQ_Diffuse"))
            (:NewEnumerator12
              (LocalVariables|SetNewTexture "/Game/CardDeck/2ColorCards/726X1044/Deck2/T_2ColorCards_Deck2_HighRes_HeartsK_Diffuse.T_2ColorCards_Deck2_HighRes_HeartsK_Diffuse"))))
        (:NewEnumerator3
          ;[0.15 0.15 0.15 0.5] Diamonds
          (switch Utilities|FlowControl|Switch|SwitchonE_CardRank (Variables|Default|GetRank)
            (:NewEnumerator0
              (LocalVariables|SetNewTexture "/Game/CardDeck/2ColorCards/726X1044/Deck2/T_2ColorCards_Deck2_HighRes_DiamondsA_Diffuse.T_2ColorCards_Deck2_HighRes_DiamondsA_Diffuse"))
            (:NewEnumerator1
              (LocalVariables|SetNewTexture "/Game/CardDeck/2ColorCards/726X1044/Deck2/T_2ColorCards_Deck2_HighRes_Diamonds2_Diffuse.T_2ColorCards_Deck2_HighRes_Diamonds2_Diffuse"))
            (:NewEnumerator2
              (LocalVariables|SetNewTexture "/Game/CardDeck/2ColorCards/726X1044/Deck2/T_2ColorCards_Deck2_HighRes_Diamonds3_Diffuse.T_2ColorCards_Deck2_HighRes_Diamonds3_Diffuse"))
            (:NewEnumerator3
              (LocalVariables|SetNewTexture "/Game/CardDeck/2ColorCards/726X1044/Deck2/T_2ColorCards_Deck2_HighRes_Diamonds4_Diffuse.T_2ColorCards_Deck2_HighRes_Diamonds4_Diffuse"))
            (:NewEnumerator4
              (LocalVariables|SetNewTexture "/Game/CardDeck/2ColorCards/726X1044/Deck2/T_2ColorCards_Deck2_HighRes_Diamonds5_Diffuse.T_2ColorCards_Deck2_HighRes_Diamonds5_Diffuse"))
            (:NewEnumerator5
              (LocalVariables|SetNewTexture "/Game/CardDeck/2ColorCards/726X1044/Deck2/T_2ColorCards_Deck2_HighRes_Diamonds6_Diffuse.T_2ColorCards_Deck2_HighRes_Diamonds6_Diffuse"))
            (:NewEnumerator6
              (LocalVariables|SetNewTexture "/Game/CardDeck/2ColorCards/726X1044/Deck2/T_2ColorCards_Deck2_HighRes_Diamonds7_Diffuse.T_2ColorCards_Deck2_HighRes_Diamonds7_Diffuse"))
            (:NewEnumerator7
              (LocalVariables|SetNewTexture "/Game/CardDeck/2ColorCards/726X1044/Deck2/T_2ColorCards_Deck2_HighRes_Diamonds8_Diffuse.T_2ColorCards_Deck2_HighRes_Diamonds8_Diffuse"))
            (:NewEnumerator8
              (LocalVariables|SetNewTexture "/Game/CardDeck/2ColorCards/726X1044/Deck2/T_2ColorCards_Deck2_HighRes_Diamonds9_Diffuse.T_2ColorCards_Deck2_HighRes_Diamonds9_Diffuse"))
            (:NewEnumerator9
              (LocalVariables|SetNewTexture "/Game/CardDeck/2ColorCards/726X1044/Deck2/T_2ColorCards_Deck2_HighRes_Diamonds10_Diffuse.T_2ColorCards_Deck2_HighRes_Diamonds10_Diffuse"))
            (:NewEnumerator10
              (LocalVariables|SetNewTexture "/Game/CardDeck/2ColorCards/726X1044/Deck2/T_2ColorCards_Deck2_HighRes_DiamondsJ_Diffuse.T_2ColorCards_Deck2_HighRes_DiamondsJ_Diffuse"))
            (:NewEnumerator11
              (LocalVariables|SetNewTexture "/Game/CardDeck/2ColorCards/726X1044/Deck2/T_2ColorCards_Deck2_HighRes_DiamondsQ_Diffuse.T_2ColorCards_Deck2_HighRes_DiamondsQ_Diffuse"))
            (:NewEnumerator12
              (LocalVariables|SetNewTexture "/Game/CardDeck/2ColorCards/726X1044/Deck2/T_2ColorCards_Deck2_HighRes_DiamondsK_Diffuse.T_2ColorCards_Deck2_HighRes_DiamondsK_Diffuse"))))))
    (:then_1
      (Rendering|Material|SetTextureParameterValue (Variables|Default|GetCardFaceMaterial) "CardFace_Texture" (LocalVariables|GetNewTexture)))))