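; BP_AI is a computer-controlled player in a slap-based card game, implementing BPI_CardPlayer events and working through the level's BP_Dealer.
; Tick watches for a change in the dealer's top card, then decides whether to slap and whether it is its turn.
; Slaps are probabilistic, including occasional false slaps, and both slaps and plays use randomized reaction delays.
; Won cards go face-down into the bottom of its deck, and losing stops its Tick logic.
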(event Custom|HandleAITurn
  ;[0.15 0.15 0.15 0.5] AI Handle Functions
  (Utilities|FlowControl|Delay (Math|Random|RandomFloatinRange 0.8 1.2))
  (CallFunction|PlayTurn))

(event Custom|HandleAISlap
  ;[0.15 0.15 0.15 0.5] AI Handle Functions
  (Utilities|FlowControl|Delay (Math|Random|RandomFloatinRange 0.2 0.5))
  (Default|PlayerSlap (Variables|Default|GetDealer) self))

(event Custom|PlayTurn
  (bind _deck (Variables|Default|GetDeck))
  (bind _deck_2 (Variables|Default|GetDeck))
  ;[0.15 0.15 0.15 0.5] Play Turn
  (if (> (Utilities|Array|Length (Variables|Default|GetDeck)) 0)
    (bind _wasplayerturn (Default|PlayPlayerTurn (Variables|Default|GetDealer) self (Utilities|Array|Get(acopy) _deck (Utilities|Array|LastIndex _deck))))
    (if _wasplayerturn
      (Utilities|Array|RemoveIndex _deck_2 (Utilities|Array|LastIndex _deck_2)))))

(event EventBeginPlay
  ;[0.15 0.15 0.15 0.5] Setup
  (bind _outactors (Actor|GetAllActorsOfClass "/Game/GameAssets/Blueprints/Dealer/BP_Dealer.BP_Dealer_C" :!label _label))
  (bind _output_get (Variables|Default|SetDealer (Utilities|Array|Get(acopy) _outactors)))
  (Utilities|IsValid _output_get
    (:Is%20Not%20Valid
      (goto _label))))

(event EventTick
  (params (DeltaSeconds :type Float%20%28single-precision%29))
  (bind _dealer (Variables|Default|GetDealer))
  (bind _deck (Variables|/Game/GameAssets/Blueprints/Dealer/BP_Dealer.BP_Dealer_C|GetDeck _dealer))
  (bind _returnvalue (Utilities|Array|LastIndex _deck))
  (bind _output (Utilities|Array|Get(acopy) _deck _returnvalue))
  (if (not (Variables|Default|GetLost))
    (if (or (== 0 (Variables|Default|GetLastCardPlayed)) (!= (Variables|Default|GetLastCardPlayed) _output))
      (Variables|Default|SetLastCardPlayed _output)
      (bind _bool (CallFunction|ShouldSlap))
      (if _bool
        (CallFunction|HandleAISlap))
      (bind _bool_2 (CallFunction|IsMyTurn))
      (if _bool_2
        (CallFunction|HandleAITurn)))))

(event EventWonGame
  ;[0.15 0.15 0.15 0.5] BPI_CardPlayer Events
)

(event EventWinCards
  (params (AddedCards :type Array%20of%20BP%20Card%20Object%20References))
  ;[0.15 0.15 0.15 0.5] BPI_CardPlayer Events
  (for (_array_element _array_index) AddedCards
    (Utilities|Array|Insert (Variables|Default|GetDeck) _array_element _array_index)
    (Default|MovetoPosition _array_element (Variables|Default|GetDeckPosition) _array_index)
    (Default|FlipCardDown _array_element)
    (Default|OrienttoLocation _array_element (Variables|Default|GetDeckPosition) (Variables|/Game/GameAssets/Blueprints/Dealer/BP_Dealer.BP_Dealer_C|GetDealerDeckPosition (Variables|Default|GetDealer))))
  (CallFunction|ResetDeckCardsPositions))

(event EventLostGame
  ;[0.15 0.15 0.15 0.5] BPI_CardPlayer Events
  (Variables|Default|SetLost true)
  (Development|PrintString (Utilities|String|Append "AI " (Utilities|GetDisplayName 0) " is eliminated from the game") true true "(R=0.371088,G=0.248545,B=1.000000,A=1.000000)" 1e+01))

(fn ConstructionScript)

(fn IsMyTurn
  (bind _dealer (Variables|Default|GetDealer))
  (bind _dealer_2 (Variables|Default|GetDealer))
  (if (Math|Boolean|ANDBoolean (== (Utilities|Array|Get(acopy) (Variables|/Game/GameAssets/Blueprints/Dealer/BP_Dealer.BP_Dealer_C|GetPlayers _dealer) (Variables|/Game/GameAssets/Blueprints/Dealer/BP_Dealer.BP_Dealer_C|GetPlayerTurnNumber _dealer)) self) (not (Variables|/Game/GameAssets/Blueprints/Dealer/BP_Dealer.BP_Dealer_C|GetWaitingToGiveCards _dealer_2)) (Variables|/Game/GameAssets/Blueprints/Dealer/BP_Dealer.BP_Dealer_C|GetHasGameStarted _dealer_2))
    (return true)
    (else
      (return false))))

(fn ResetDeckCardsPositions
  (for (_array_element _array_index) (Variables|Default|GetDeck)
    (Default|MovetoPosition _array_element (Variables|Default|GetDeckPosition) _array_index)))

(fn ShouldSlap
  (if (Variables|/Game/GameAssets/Blueprints/Dealer/BP_Dealer.BP_Dealer_C|GetHasGameStarted (Variables|Default|GetDealer))
    (bind _slappable (Default|IsDeckSlappable (Variables|Default|GetDealer)))
    (if _slappable
      (if (>= (Math|Random|RandomFloatinRange 0.0 1e+02) 5e+01)
        (return true)
        (else
          (return false)))
      (elif (>= (Math|Random|RandomFloatinRange 0.0 1e+02) 95.0)
        (return true)
        (else
          (return false))))
    (else
      (return false))))

(fn GetDeckSize
  (return (Utilities|Array|Length (Variables|Default|GetDeck))))