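; Human player for a slap-style card game, handling mouse input and holding the player's deck while BP_Dealer runs turns and rules.
; Tick highlights hovered deck cards, drags the grabbed top card along a cursor ray intersected with the dealer deck's height, and detects the slap zone.
; Click grabs or slaps; dropping near the dealer's deck on the player's turn plays the card, otherwise it returns.
; Interface events collect won cards and quit after a win or loss.
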(event Custom|PlayTurn
  (bind _deck (Variables|Default|GetDeck))
  (bind _deck_2 (Variables|Default|GetDeck))
  (bind _returnvalue (Utilities|Array|LastIndex _deck_2))
  ;[0.15 0.15 0.15 0.5] Play Turn
  (if (> (Utilities|Array|Length (Variables|Default|GetDeck)) 0)
    (bind _wasplayerturn (Default|PlayPlayerTurn (Variables|Default|GetDealer) self (Utilities|Array|Get(acopy) _deck (Utilities|Array|LastIndex _deck))))
    (if _wasplayerturn
      ;;[0.15 0.15 0.15 0.5] Remove hover
      (Rendering|Material|SetOverlayMaterial (Variables|/Game/GameAssets/Blueprints/Cards/BP_Card.BP_Card_C|GetCardBack (Utilities|Array|Get(acopy) _deck_2 _returnvalue)) 0 :!class /Script/Engine.MeshComponent)
      (Utilities|Array|RemoveIndex _deck_2 _returnvalue))))

(event Input|EnhancedActionEvents|EnhancedInputActionIA_Click
  (params (ActionValue :type Boolean) (ElapsedSeconds :type Float%20%28double-precision%29) (TriggeredSeconds :type Float%20%28double-precision%29) (InputAction :type Input%20Action%20Object%20Reference :default "/Game/GameAssets/Blueprints/Player/Inputs/IA_Click.IA_Click"))
  ;[0.15 0.15 0.15 0.5] Grab a card
  (if (Variables|/Game/GameAssets/Blueprints/Dealer/BP_Dealer.BP_Dealer_C|GetHasGameStarted (Variables|Default|GetDealer))
    (if (Variables|Default|GetCursorOnDeck)
      (Variables|Default|SetHoldingCard true)
      (elif (Variables|Default|GetCanSlap)
        (Default|PlayerSlap (Variables|Default|GetDealer) self)
        (Development|PrintString "Slap !")))))

(event Input|EnhancedActionEvents|EnhancedInputActionIA_Drop
  (params (ActionValue :type Boolean) (ElapsedSeconds :type Float%20%28double-precision%29) (TriggeredSeconds :type Float%20%28double-precision%29) (InputAction :type Input%20Action%20Object%20Reference :default "/Game/GameAssets/Blueprints/Player/Inputs/IA_Drop.IA_Drop"))
  (bind (_card _decklenght) (CallFunction|GetDeckLastIndex))
  (bind _dealer (Variables|Default|GetDealer))
  ;[0.15 0.15 0.15 0.5] Release the grabbed card
  (if (Variables|Default|GetHoldingCard)
    (if (<= (Math|Vector|Distance(Vector) (Variables|/Game/GameAssets/Blueprints/Dealer/BP_Dealer.BP_Dealer_C|GetDealerDeckPosition (Variables|Default|GetDealer)) (Transformation|GetActorLocation _card)) 4e+01)
      (Utilities|Casting|CastToBP_Player (Utilities|Array|Get(acopy) (Variables|/Game/GameAssets/Blueprints/Dealer/BP_Dealer.BP_Dealer_C|GetPlayers _dealer) (Variables|/Game/GameAssets/Blueprints/Dealer/BP_Dealer.BP_Dealer_C|GetPlayerTurnNumber _dealer))
        (:then
          (CallFunction|PlayTurn))
        (:CastFailed
          (Default|MovetoPosition _card (Variables|Default|GetDeckPosition) _decklenght :!label _label)))
      (else
        (goto _label)))
    (Variables|Default|SetHoldingCard false)))

(event EventBeginPlay
  (bind _returnvalue (Game|GetPlayerController 0))
  ;[0.15 0.15 0.15 0.5] Setup
  (bind _outactors (Actor|GetAllActorsOfClass "/Game/GameAssets/Blueprints/Dealer/BP_Dealer.BP_Dealer_C" :!label _label))
  (bind _output_get (Variables|Default|SetDealer (Utilities|Array|Get(acopy) _outactors)))
  (Utilities|IsValid _output_get
    (:Is%20Valid
      (Utilities|FlowControl|DelayUntilNextTick)
      (Input|AddMappingContext (PlayerController|LocalPlayerSubsystems|GetEnhancedInputLocalPlayerSubsystem _returnvalue) "/Game/GameAssets/Blueprints/Player/Inputs/IMC_Player.IMC_Player" 0 "(bIgnoreAllPressedKeysUntilRelease=True,bForceImmediately=False,bNotifyUserSettings=False)")
      (Variables|/Script/Engine.PlayerController|SetbShowMouseCursor _returnvalue true))
    (:Is%20Not%20Valid
      (goto _label))))

(event EventTick
  (params (DeltaSeconds :type Float%20%28single-precision%29))
  (bind (_card _decklenght) (CallFunction|GetDeckLastIndex))
  ;[0.15 0.15 0.15 0.5] Event tick
  (Utilities|FlowControl|Sequence
    (:then_0
      ;[0.15 0.15 0.15 0.5] Deck highlighting when hovering
      (for _array_element (Variables|Default|GetDeck)
        (if (== (.hitactor (.HitResult (Game|Player|GetHitResultUnderCursorbyChannel (Game|GetPlayerController 0) "TraceTypeQuery1" true))) _array_element)
          (Rendering|Material|SetOverlayMaterial (Variables|/Game/GameAssets/Blueprints/Cards/BP_Card.BP_Card_C|GetCardBack _array_element) "/Game/GameAssets/Assets/Materials/M_Highlight.M_Highlight" :!class /Script/Engine.MeshComponent)
          (Variables|Default|SetCursorOnDeck true)
          (else
            (Rendering|Material|SetOverlayMaterial (Variables|/Game/GameAssets/Blueprints/Cards/BP_Card.BP_Card_C|GetCardBack _array_element) 0 :!class /Script/Engine.MeshComponent)
            (Variables|Default|SetCursorOnDeck false)))))
    (:then_1
      ;[0.15 0.15 0.15 0.5] Set grabbed card's position
      (if (Variables|Default|GetHoldingCard)
        (bind _output_get (Variables|/Game/GameAssets/Blueprints/Cards/BP_Card.BP_Card_C|SetTargetLocation _card (CallFunction|OnGrabNewPosition)))
        (Default|MovetoPosition _card _output_get _decklenght)))
    (:then_2
      ;[0.15 0.15 0.15 0.5] Check if in slap zone
      (if (== (.hitcomponent (.HitResult (Game|Player|GetHitResultUnderCursorbyChannel (Game|GetPlayerController 0) "TraceTypeQuery1" true))) (Variables|/Game/GameAssets/Blueprints/Dealer/BP_Dealer.BP_Dealer_C|GetSlapZone (Variables|Default|GetDealer)))
        (Variables|Default|SetCanSlap true)
        (else
          (Variables|Default|SetCanSlap false))))))

(event EventWonGame
  ;[0.15 0.15 0.15 0.5] BPI_CardPlayer Events
  (Development|PrintString "Won the game ! Exiting in 5 seconds" true true "(R=0.371088,G=0.248545,B=1.000000,A=1.000000)" 1e+01)
  (Utilities|FlowControl|Delay 5.0)
  (Game|QuitGame 0 "Quit" false))

(event EventWinCards
  (params (AddedCards :type Array%20of%20BP%20Card%20Object%20References))
  ;[0.15 0.15 0.15 0.5] BPI_CardPlayer Events
  (for _array_element AddedCards
    (Utilities|Array|Add (Variables|Default|GetDeck) _array_element)
    (Default|MovetoPosition _array_element (Variables|Default|GetDeckPosition) (Utilities|Array|Length (Variables|Default|GetDeck)))
    (Default|FlipCardDown _array_element)
    (Default|OrienttoLocation _array_element (Variables|Default|GetDeckPosition) (Variables|/Game/GameAssets/Blueprints/Dealer/BP_Dealer.BP_Dealer_C|GetDealerDeckPosition (Variables|Default|GetDealer)))))

(event EventLostGame
  ;[0.15 0.15 0.15 0.5] BPI_CardPlayer Events
  (Development|PrintString "Lost the game ! Exiting in 5 seconds" true true "(R=0.371088,G=0.248545,B=1.000000,A=1.000000)" 1e+01)
  (Utilities|FlowControl|Delay 5.0)
  (Game|QuitGame 0 "Quit" false))

(fn ConstructionScript)

(fn OnGrabNewPosition
  (bind _returnvalue (Game|GetPlayerController 0))
  (bind (_locationx _locationy) (Game|Player|GetMousePosition _returnvalue))
  (bind (_worldposition _worlddirection) (Class|GameplayStatics|DeprojectScreentoWorld _returnvalue (Math|Vector2D|MakeVector2D _locationx _locationy)))
  (return (+ (Math|Vector|MakeVector (.x _worldposition) (.y _worldposition) (.z _worldposition)) (* (Math|Vector|MakeVector (.x _worlddirection) (.y _worlddirection) (.z _worlddirection)) (/ (- (.z (Variables|/Game/GameAssets/Blueprints/Dealer/BP_Dealer.BP_Dealer_C|GetDealerDeckPosition (Variables|Default|GetDealer))) (.z _worldposition)) (.z _worlddirection))))))

(fn GetDeckLastIndex
  (bind _deck (Variables|Default|GetDeck))
  (return (Utilities|Array|Get(acopy) _deck (Utilities|Array|LastIndex _deck)) (Utilities|Array|Length (Variables|Default|GetDeck))))

(fn GetDeckSize
  (return (Utilities|Array|Length (Variables|Default|GetDeck))))