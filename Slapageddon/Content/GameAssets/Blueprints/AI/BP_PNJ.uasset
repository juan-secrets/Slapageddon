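; BP_PNJ is an NPC Blueprint whose character look and pose are set per placed instance, with no runtime logic in its empty BeginPlay.
; The construction script calls SetSkeletalMesh, which uses an index to pick a cowboy, bandit or masked-up bandit mesh.
; A sitting flag then selects that character's main or idle animation Blueprint, with both bandit variants sharing the same pair.
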(event EventBeginPlay
  ;[0.15 0.15 0.15 0.5] Setup
)

(fn ConstructionScript
  (CallFunction|SetSkeletalMesh))

(fn SetSkeletalMesh
  (switch int (Variables|Default|GetSkeletalMeshIndex)
    (:0
      (Components|SkeletalMesh|SetSkeletalMeshAsset (Variables|Character|GetMesh) "/Game/Cowboy_character/Mesh/SM_SkeletalMesh_cowboy_character.SM_SkeletalMesh_cowboy_character")
      (if (Variables|Default|GetIsSitting)
        (Components|SkeletalMesh|SetAnimInstanceClass (Variables|Character|GetMesh) "/Game/GameAssets/Assets/Animation/ABP_Cowboy.ABP_Cowboy_C")
        (else
          (Components|SkeletalMesh|SetAnimInstanceClass (Variables|Character|GetMesh) "/Game/GameAssets/Assets/Animation/ABP_Cowboy_Idle.ABP_Cowboy_Idle_C"))))
    (:1
      (Components|SkeletalMesh|SetSkeletalMeshAsset (Variables|Character|GetMesh) "/Game/Bandit/Mesh/BanditUnreal.BanditUnreal")
      (if (Variables|Default|GetIsSitting) :!label _label
        (Components|SkeletalMesh|SetAnimInstanceClass (Variables|Character|GetMesh) "/Game/GameAssets/Assets/Animation/ABP_Bandit.ABP_Bandit_C")
        (else
          (Components|SkeletalMesh|SetAnimInstanceClass (Variables|Character|GetMesh) "/Game/GameAssets/Assets/Animation/ABP_Bandit_Idle.ABP_Bandit_Idle_C"))))
    (:2
      (Components|SkeletalMesh|SetSkeletalMeshAsset (Variables|Character|GetMesh) "/Game/Bandit/Skins/BanditMaskUp.BanditMaskUp")
      (goto _label))))