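; BP_TurnIndicator is a turn indicator actor that glides toward whatever location and rotation it is given.
; MoveToPosition and RotateOnPosition only store the targets, and Tick applies them every frame.
; Location eases in per axis with FInterpTo at MovingSpeed, while rotation turns at a steady rate through RInterpToConstant at RotationSpeed.
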(event Custom|RotateOnPosition
  (params (NewRotation :type Rotator))
  (Variables|Default|SetTargetRotation NewRotation))

(event Custom|MoveToPosition
  (params (NewLocation :type Vector))
  (Variables|Default|SetTargetLocation NewLocation))

(event EventTick
  (params (DeltaSeconds :type Float%20%28single-precision%29))
  (bind _returnvalue (Transformation|GetActorLocation))
  (bind _targetlocation (Variables|Default|GetTargetLocation))
  (Utilities|FlowControl|Sequence
    (:then_0
      ;[0.15 0.15 0.15 0.5] Update Card Location
      (Transformation|SetActorLocation (Math|Vector|MakeVector (Math|Interpolation|FInterpTo (.x _returnvalue) (.x _targetlocation) DeltaSeconds (Variables|Default|GetMovingSpeed)) (Math|Interpolation|FInterpTo (.y _returnvalue) (.y _targetlocation) DeltaSeconds (Variables|Default|GetMovingSpeed)) (Math|Interpolation|FInterpTo (.z _returnvalue) (.z _targetlocation) DeltaSeconds (Variables|Default|GetMovingSpeed))) false false))
    (:then_1
      ;[0.15 0.15 0.15 0.5] Update Card Rotation
      (Transformation|SetActorRotation (Class|KismetMathLibrary|RInterptoConstant (Transformation|GetActorRotation) (Variables|Default|GetTargetRotation) DeltaSeconds (Variables|Default|GetRotationSpeed))))))

(fn ConstructionScript)